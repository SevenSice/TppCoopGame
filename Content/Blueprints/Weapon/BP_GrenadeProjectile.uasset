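; Grenade projectile actor that explodes on a fixed timer shortly after spawning.
; On BeginPlay it waits out a short delay, then calls an Explode event that spawns the explosion particle effect at its transform.
; It then applies full radial damage without falloff, credited to its instigator's controller, draws a debug sphere showing the damage radius and destroys itself.
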(event `self.ReceiveBeginPlay`
  (bind (_returnvalue_location _returnvalue_rotation _returnvalue_scale) (`KismetMathLibrary.BreakTransform` (`self.GetTransform`)))
  (`KismetSystemLibrary.Delay` 1.0)
  (`self.Explode`)
  (`GameplayStatics.ApplyRadialDamage` :`BaseDamage` 100.0 :`Origin` _returnvalue_location :`DamageRadius` (`self.DamageRadius`) :`DamageCauser` self :`InstigatedByController` (`self.GetInstigatorController`) :`bDoFullDamage` true)
  (`KismetSystemLibrary.DrawDebugSphere` _returnvalue_location (`self.DamageRadius`) 12 (struct :`R` 1.0 :`G` 0.41357 :`A` 1.0) 1.0 1.0)
  (`self.K2_DestroyActor`))

(event `Explode`
  (bind (_returnvalue_location _returnvalue_rotation _returnvalue_scale) (`KismetMathLibrary.BreakTransform` (`self.GetTransform`)))
  (`GameplayStatics.SpawnEmitterAtLocation` "/Game/WeaponEffects/Explosion/P_Explosion.P_Explosion" _returnvalue_location (struct) _returnvalue_scale))

(fn `UserConstructionScript`)