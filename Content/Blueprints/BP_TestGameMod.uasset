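; BP_TestGameMod is a test game mode Blueprint that spawns BP_TrackerBot enemies at locations chosen by the Environment Query System.
; The SpawnNewBot event runs EQS_FindSpawnLocation with itself as querier, picking randomly from the best 25 percent of results.
; On query success, it prints the result count, then draws a debug sphere and spawns a bot at each returned location, skipping spawns whose collisions cannot be resolved.
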(event `self.SpawnNewBot`
  (bind _returnvalue (`EnvQueryManager.RunEQSQuery` "/Game/Blueprints/AI/EQS_FindSpawnLocation.EQS_FindSpawnLocation" self "RandomBest25Pct"))
  (add `EnvQueryInstanceBlueprintWrapper.OnQueryFinishedEvent` _returnvalue (delegate `OnQueryFinishedEvent_Event_0`)))

(event `OnQueryFinishedEvent_Event_0`
  (params (QueryInstance :type "EnvQueryInstanceBlueprintWrapper Object Reference") (QueryStatus :type "EEnvQueryStatus Enum" :default "Processing"))
  (bind _returnvalue (`EnvQueryInstanceBlueprintWrapper.GetResultsAsLocations` QueryInstance))
  (switch `EEnvQueryStatus` QueryStatus
    (:`Success`
      (`KismetSystemLibrary.PrintString` (`KismetStringLibrary.Conv_IntToString` (`KismetArrayLibrary.Array_Length` _returnvalue)))
      (for _array_element _returnvalue
        (`KismetSystemLibrary.DrawDebugSphere` _array_element 50.0 12 (struct :`R` 1.0 :`G` 0.467075 :`A` 1.0) 2.0 2.0)
        (`|SpawnActorFromClass` "/Game/TrackerBot/BP_TrackerBot.BP_TrackerBot_C" (`KismetMathLibrary.MakeTransform` _array_element) "AdjustIfPossibleButDontSpawnIfColliding" "OverrideRootScale" null null)))))

(fn `UserConstructionScript`)